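; BP_GridManager is an actor that builds a flat grid of BP_Tile actors when play begins.
; Nested loops over GridSizeX and GridSizeY spawn one tile per cell, placed at each index times TileSize on X and Y at zero height.
; Positions are absolute world coordinates, independent of the manager's own location, and the inclusive loop bounds may yield one extra row and column.
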(event EventBeginPlay
  (for _index (range 0 (Variables|Default|GetGridSizeX))
    (for _index_2 (range 0 (Variables|Default|GetGridSizeY))
      (Game|SpawnActorfromClass "/Game/BP_Tile/BP_Tile.BP_Tile_C" (Math|Transform|MakeTransform (Math|Vector|MakeVector (Math|Conversions|ToFloat(Integer) (* _index (Variables|Default|GetTileSize))) (Math|Conversions|ToFloat(Integer) (* _index_2 (Variables|Default|GetTileSize))) 0.0)) "Undefined" "MultiplyWithRoot" 0 0))))

(event Collision|EventActorBeginOverlap
  (params (OtherActor :type Actor%20Object%20Reference)))

(event EventTick
  (params (DeltaSeconds :type Float%20%28single-precision%29)))

(fn ConstructionScript)